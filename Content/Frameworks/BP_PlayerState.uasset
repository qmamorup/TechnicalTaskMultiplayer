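; Player state Blueprint that tracks each player's name, kill count, death count and dead flag.
; On BeginPlay, if player controller 0 is local, it loads the saved player info and passes the stored name to SendMyNameToServer, which sets MyName.
; AddKill and AddDeath events update the tallies, with AddDeath also setting IsDead.
; The deaths counter has a RepNotify function, which is empty.
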(event Custom|AddKill
  (Math|Integer|IncrementInt (Variables|Default|GetMyKills)))

(event Custom|AddDeath
  (Math|Integer|IncrementInt (Variables|Default|GetMyDeaths)
    (:%20%20
      (Variables|Default|SetIsDead true))))

(event Custom|Send%20My%20Name%20To%20Server
  (params (MyName :type Text))
  (Variables|Default|SetMyName MyName))

(event EventBeginPlay
  (if (Pawn|IsLocalPlayerController (Game|GetPlayerController 0))
    (bind _returnvalue (SaveGame|LoadGamefromSlot "Info"))
    (bind _asbp_player_save_info (Utilities|Casting|CastToBP_PlayerSaveInfo _returnvalue))
    (CallFunction|SendMyNametoServer (Variables|/Game/Start/BP_PlayerSaveInfo.BP_PlayerSaveInfo_C|GetPlayer%20Name _asbp_player_save_info))))

(event EventTick
  (params (DeltaSeconds :type Float%20%28single-precision%29)))

(fn ConstructionScript)

(fn OnRepMyDeaths)