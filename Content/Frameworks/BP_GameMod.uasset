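; Game mode that handles player respawning and relays chat-style messages to every player.
; Respawn destroys the controller's current pawn, spawns a third-person character at a random PlayerStart and possesses it.
; SendTo_GameMod loops over the game state's player array and forwards sender and message to each BP_PlayerController through OnMessageSendToGMEvent.
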(event Custom|Respawn
  (params (Controller :type Controller%20Object%20Reference))
  (bind _returnvalue (Pawn|GetControlledPawn Controller))
  (bind _outactors (Actor|GetAllActorsOfClass "/Script/Engine.PlayerStart"))
  (Utilities|IsValid _returnvalue
    (:Is%20Valid
      (Actor|DestroyActor _returnvalue))
    (:Is%20Not%20Valid
      _))
  (bind _returnvalue_2 (Game|SpawnActorfromClass "/Game/ThirdPerson/Blueprints/BP_ThirdPersonCharacter.BP_ThirdPersonCharacter_C" (Transformation|GetActorTransform (Utilities|Array|Get(acopy) _outactors (Math|Random|RandomIntegerinRange 0 (- (Utilities|Array|Length _outactors) 1)))) "AdjustIfPossibleButAlwaysSpawn" 0 0))
  (Pawn|Possess Controller _returnvalue_2))

(event Custom|SendTo_GameMod
  (params (Sender :type String) (Message :type String))
  (for _array_element (Variables|/Script/Engine.GameStateBase|GetPlayerArray (Game|GetGameState))
    (bind _asbp_player_controller (Utilities|Casting|CastToBP_PlayerController (Game|GetPlayerController _array_element)))
    (Default|OnMessageSendtoGMEvent _asbp_player_controller Sender Message)))

(event EventBeginPlay)

(event EventTick
  (params (DeltaSeconds :type Float%20%28single-precision%29)))

(fn ConstructionScript)