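; Player controller that handles UI input, chat messaging and the player's character gender.
; On authority possession it reads the saved sex from the "Info" slot and passes it through ServerChangeSex to the pawn.
; Menu, scoreboard and chat inputs drive BP_HUD widgets, with menu and chat toggling cursor and pawn input.
; Relay events forward messages to GameState and GameMode and rebroadcast those returning from GameMode through a dispatcher.
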(event Custom|Local%20Change%20sex
  (bind _returnvalue (SaveGame|LoadGamefromSlot "Info"))
  (bind _asbp_player_save_info (Utilities|Casting|CastToBP_PlayerSaveInfo _returnvalue))
  (CallFunction|ServerChangeSex (Variables|/Game/Start/BP_PlayerSaveInfo.BP_PlayerSaveInfo_C|GetPlayer%20Sex _asbp_player_save_info)))

(event Custom|Server%20Change%20Sex
  (params (Gender :type Boolean))
  (bind _asbp_third_person_character (Utilities|Casting|CastToBP_ThirdPersonCharacter (Pawn|GetControlledPawn)))
  (Variables|/Game/ThirdPerson/Blueprints/BP_ThirdPersonCharacter.BP_ThirdPersonCharacter_C|SetGender _asbp_third_person_character Gender))

(event Custom|SendTo_PlayerController-GS
  (params (Sender :type String) (Message :type String))
  ;[1 1 1] to GameState
  (bind _asbp_game_state (Utilities|Casting|CastToBP_GameState (Game|GetGameState)))
  (Default|OnMessageSendtoGSEvent _asbp_game_state Sender Message))

(event Custom|HideChat
  ;[1 1 1] Show or Hide Chat
  (Default|HideChat (Variables|/Game/UI/Chat/ChatOnScreen.ChatOnScreen_C|GetChatBOX (Variables|/Game/UI/BP_HUD.BP_HUD_C|GetChatOnScreen (Variables|Default|GetAs%20BP%20HUD))))
  (Variables|Default|SetbShowMouseCursor false)
  (Input|SetInputModeGameOnly self false)
  (Input|EnableInput (Pawn|GetControlledPawn) self))

(event Custom|OnMessageSendToGM_Event
  (params (Sender :type String) (Message :type String))
  ;[1 1 1] from GameMode
  (Default|CallOnMessageSendtoGM Sender Message))

(event Custom|SendTo_PlayerController-GM
  (params (Sender :type String) (Message :type String))
  ;[1 1 1] to GameMode
  (bind _asbp_game_mod (Utilities|Casting|CastToBP_GameMod (Game|GetGameMode)))
  (Default|SendtoGameMod _asbp_game_mod Sender Message))

(event EventBeginPlay
  (Input|SetInputModeGameOnly self false)
  (bind _asbp_hud (Utilities|Casting|CastToBP_HUD (HUD|GetHUD)))
  (Variables|Default|SetAs%20BP%20HUD _asbp_hud))

(event EventTick
  (params (DeltaSeconds :type Float%20%28single-precision%29)))

(event EventPossess
  (params (PossessedPawn :type Pawn%20Object%20Reference))
  (Networking|SwitchHasAuthority
    (:Authority
      (CallFunction|LocalChangeSex))))

(event Input|ActionEvents|InputActionMainMenu
  (params (Key :type Key%20Structure :default "None"))
  (bind _returnvalue (Pawn|GetControlledPawn))
  (bind _self self)
  (bind _as_bp_hud (Variables|Default|GetAs%20BP%20HUD))
  ;[1 1 1] If Chat is opened
  (:Pressed
    (if (== (Variables|/Script/UMG.WidgetSwitcher|GetActiveWidgetIndex (Variables|/Game/UI/Chat/ChatBOX.ChatBOX_C|GetWidgetSwitcher_0 (Variables|/Game/UI/Chat/ChatOnScreen.ChatOnScreen_C|GetChatBOX (Variables|/Game/UI/BP_HUD.BP_HUD_C|GetChatOnScreen (Variables|Default|GetAs%20BP%20HUD))))) 1)
      (CallFunction|HideChat)
      (else
        (Utilities|FlowControl|FlipFlop
          (:A
            (Default|DrawMainMenu _as_bp_hud)
            (Variables|Default|SetbShowMouseCursor true)
            (Input|DisableInput _returnvalue _self))
          (:B
            (Default|DeleteMainMenu _as_bp_hud)
            (Variables|Default|SetbShowMouseCursor false)
            (Input|EnableInput _returnvalue _self)))))))

(event Input|ActionEvents|InputActionScoreBoard
  (params (Key :type Key%20Structure :default "None"))
  (bind _as_bp_hud (Variables|Default|GetAs%20BP%20HUD))
  (:Pressed
    (Default|ShowScoreBoard _as_bp_hud))
  (:Released
    (Default|CloseScoreBoard _as_bp_hud)))

(event Input|ActionEvents|InputActionChat
  (params (Key :type Key%20Structure :default "None"))
  (bind _returnvalue (Pawn|GetControlledPawn))
  (bind _self self)
  (bind _self_2 self)
  (bind _as_bp_hud (Variables|Default|GetAs%20BP%20HUD))
  (bind _chatonscreen (Variables|/Game/UI/BP_HUD.BP_HUD_C|GetChatOnScreen _as_bp_hud))
  (bind _chatbox (Variables|/Game/UI/Chat/ChatOnScreen.ChatOnScreen_C|GetChatBOX _chatonscreen))
  ;[1 1 1] Show or Hide Chat
  (:Pressed
    (if (== (Variables|/Script/UMG.WidgetSwitcher|GetActiveWidgetIndex (Variables|/Game/UI/Chat/ChatBOX.ChatBOX_C|GetWidgetSwitcher_0 _chatbox)) 0)
      (Default|ShowChat _chatbox)
      (Variables|Default|SetbShowMouseCursor true)
      (Input|SetInputModeGameandUI _self_2 (Variables|/Game/UI/Chat/ChatBOX.ChatBOX_C|GetChatLine _chatbox) "DoNotLock" true false)
      (Input|DisableInput _returnvalue _self)
      (else
        (Default|HideChat _chatbox)
        (Variables|Default|SetbShowMouseCursor false)
        (Input|SetInputModeGameOnly _self_2 false)
        (Input|EnableInput _returnvalue _self)))))

(fn ConstructionScript)

(fn SetMesh
  (params (Gender :type Boolean))
  (CallFunction|ServerChangeSex Gender))